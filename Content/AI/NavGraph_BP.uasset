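; Navigation graph actor that builds a waypoint path between actors S and T on BeginPlay and can spawn attached NavPoint_BP children.
; FindClosestNavPoint locates each end's nav point by repeated sphere traces with a growing radius, which is never reset between searches.
; GeneratePath, defined outside these graphs, links the two points, and Path stores their locations bracketed by source and destination.
; The DFS function is an empty stub.
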(event EventBeginPlay
  (CallFunction|FindPathtoTarget (Transformation|GetActorLocation (Variables|Default|GetS)) (Transformation|GetActorLocation (Variables|Default|GetT))))

(event Collision|EventActorBeginOverlap
  (params (OtherActor :type Actor%20Object%20Reference)))

(event EventTick
  (params (DeltaSeconds :type Float%20%28single-precision%29)))

(fn ConstructionScript)

(fn CreateNavPoint
  (bind _self self)
  (bind _returnvalue (Game|SpawnActorfromClass "/Game/AI/NavPoint_BP.NavPoint_BP_C" (Transformation|GetActorTransform) "AlwaysSpawn" _self 0))
  (Transformation|AttachActorToActor _returnvalue _self "None" "KeepWorld" "KeepRelative" "KeepRelative" true))

(fn FindPathtoTarget
  (params (Source :type Vector) (Destination :type Vector))
  (bind _path (Variables|Default|GetPath))
  (bind _path_2 (Variables|Default|GetPath))
  (Utilities|Array|Clear _path)
  (Utilities|Array|Add _path Source)
  (bind _np (CallFunction|FindClosestNavPoint Source))
  (Variables|Default|SetSourceNavPoint _np)
  (bind _np_2 (CallFunction|FindClosestNavPoint Destination))
  (Variables|Default|SetDestNavPoint _np_2)
  (bind _returnvalue (Class|NavGraph|GeneratePath (Variables|Default|GetSourceNavPoint) (Variables|Default|GetDestNavPoint)))
  (for _array_element _returnvalue
    (Utilities|Array|Add _path_2 (Transformation|GetActorLocation _array_element)))
  (Utilities|Array|Add _path_2 Destination))

(fn FindClosestNavPoint
  (params (Location :type Vector))
  (Variables|Default|SetTraceFound false)
  (while (not (Variables|Default|GetTraceFound))
    (bind (_outhit _returnvalue) (Collision|SphereTraceForObjects Location (+ Location "1.000000, 0,0.000000") (Variables|Default|GetTraceRadius) (Utilities|Array|MakeArray "ObjectTypeQuery8") true 0 "ForOneFrame"))
    (if _returnvalue
      (bind _asnav_point (Utilities|Casting|CastToNavPoint (.HitActor (Collision|BreakHitResult _outhit))))
      (Variables|Default|SetTraceFound true)
      (return _asnav_point)
      (else
        (Variables|Default|SetTraceRadius (+ (Variables|Default|GetTraceRadius) 1e+01))))))

(fn DFS)