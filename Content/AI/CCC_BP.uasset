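; CCC_BP is an AI pawn Blueprint built to seek out PostCollecton_BP actors, but its search-and-move chain is disconnected, so never runs.
; Construction caches the level's NavMeshBoundsVolume, whose X extent caps the search radius.
; FindPCBox grows a debug-drawn sphere trace per call until it finds a target for AIMoveTo.
; Targets reached within a set distance join an ignore list and are cleared.
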(event EventBeginPlay
  (|CallParentFunction) ; This node is disabled and will not be called.\nDrag off pins to build functionality.
)

(event Collision|EventActorBeginOverlap
  (params (OtherActor :type Actor%20Object%20Reference))
  (|CallParentFunction OtherActor) ; This node is disabled and will not be called.\nDrag off pins to build functionality.
)

(event EventTick
  (params (DeltaSeconds :type Float%20%28single-precision%29))
  (|CallParentFunction DeltaSeconds))

(fn ConstructionScript
  (|CallParentFunction)
  (bind _returnvalue (Actor|GetActorOfClass "/Script/NavigationSystem.NavMeshBoundsVolume"))
  (Utilities|IsValid _returnvalue
    (:Is%20Valid
      (Variables|Default|SetLevelNavMesh _returnvalue))))

(fn FindPCBox
  (bind _returnvalue (Transformation|GetActorLocation))
  (Utilities|IsValid (Variables|Default|GetTargetBox)
    (:Is%20Valid
      (if (< (Math|Vector|VectorLength (- (Transformation|GetActorLocation (Variables|Default|GetTargetBox)) (Transformation|GetActorLocation))) 3e+02)
        (Utilities|Array|Add (Variables|Default|GetTest) (Variables|Default|GetTargetBox))
        (Variables|Default|SetTargetBox 0)))
    (:Is%20Not%20Valid
      (bind _output_get (Variables|Default|SetTraceradius (+ (Variables|Default|GetTraceradius) 5.0)))
      (if (> _output_get (.x (.BoxExtent (Collision|GetActorBounds (Variables|Default|GetLevelNavMesh) false false))))
        (Variables|Default|SetTraceradius 0.0))
      (bind _outhit (Collision|SphereTraceForObjects _returnvalue (+ _returnvalue "1.000000, 0, 0") (Variables|Default|GetTraceradius) (Utilities|Array|MakeArray "ObjectTypeQuery7") true (Variables|Default|GetTest) "ForOneFrame"))
      (bind _aspost_collecton_bp (Utilities|Casting|CastToPostCollecton_BP (.HitActor (Collision|BreakHitResult _outhit))))
      (Variables|Default|SetTargetBox _aspost_collecton_bp)
      (Variables|Default|SetTraceradius 0.0))))